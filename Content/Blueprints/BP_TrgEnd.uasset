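; BP_TrgEnd is an end-of-game trigger that plays effects and then quits the game when its collision component is overlapped.
; BeginPlay hides its sprite component.
; On overlap, a Sequence starts two explosions at once, two spark effects (Etincelles) after a short delay, and Quit Game after a longer one.
; The overlap has no actor filter or one-shot guard.
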(event OnComponentBeginOverlap(CollisionComponent)
  (params (OverlappedComponent :type Primitive%20Component%20Object%20Reference) (OtherActor :type Actor%20Object%20Reference) (OtherComp :type Primitive%20Component%20Object%20Reference) (OtherBodyIndex :type Integer) (bFromSweep :type Boolean) (SweepResult :type Hit%20Result%20Structure%20%28by%20ref%29))
  (Utilities|FlowControl|Sequence
    (:then_0
      (Components|Activation|Activate (Variables|Default|GetExplosion1) false)
      (Components|Activation|Activate (Variables|Default|GetExplosion2) false))
    (:then_1
      (Utilities|FlowControl|Delay 1.0)
      (Components|Activation|Activate (Variables|Default|GetEtincelles1) false)
      (Components|Activation|Activate (Variables|Default|GetEtincelles2) false))
    (:then_2
      (Utilities|FlowControl|Delay 5.0)
      (Game|QuitGame 0 "Quit"))))

(event EventBeginPlay
  (Rendering|SetVisibility (Variables|Default|GetSpriteComponent) false false))

(event EventTick
  (params (DeltaSeconds :type Float%20%28single-precision%29)))

(fn ConstructionScript)